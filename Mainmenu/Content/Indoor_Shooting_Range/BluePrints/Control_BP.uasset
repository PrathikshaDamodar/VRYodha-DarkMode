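; Shooting range control panel that sets a distance in meters and moves itself to it, likely as the target carrier.
; Interact compares the hit component: Up and Down step the clamped Distance and refresh the Meters text.
; Hitting Sponge offsets the Cube's starting location along the control actor's forward vector by that distance, then a Timeline lerps this actor there from its current location.
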(event `CustomEvent_0`
  (set `self.new location` (`self.K2_GetActorLocation` (`self.cube ?`)) :!label _label))

(event `self.ReceiveBeginPlay`
  (bind _returnvalue (`self.K2_GetActorLocation` (`self.cube ?`)))
  (set `self.NewVar_0` (.x _returnvalue))
  (set `self.default location` _returnvalue)
  (goto _label))

(event `/Game/Indoor_Shooting_Range/BluePrints/BP_ExampleInterface.Interact`
  (params (Hit :type "HitResult Structure"))
  (bind (_bblockinghit _binitialoverlap _time _distance _location _impactpoint _normal _impactnormal _physmat _hitactor _hitcomponent) (`GameplayStatics.BreakHitResult` Hit))
  ;[1 0 0.3047] Up button
  (if (== (`self.up`) _hitcomponent)
    (bind _output_get (set `self.distance` (`KismetMathLibrary.Clamp` (+ (`self.distance`) 1) 0 (`self.MaxDistance`))))
    (`TextRenderComponent.K2_SetText` (`self.Meters`) (`KismetTextLibrary.Conv_IntToText` _output_get))
    (else
      ;[1 0.7266 0] Down button
      (if (== (`self.down`) _hitcomponent)
        (bind _output_get_2 (set `self.distance` (`KismetMathLibrary.Clamp` (- (`self.distance`) 1) 0 (`self.MaxDistance`))))
        (`TextRenderComponent.K2_SetText` (`self.Meters`) (`KismetTextLibrary.Conv_IntToText` _output_get_2))
        (elif (== (`self.sponge`) _hitcomponent)
          (bind _output_get_3 (set `self.new location` (+ (`self.default location`) (* (`self.GetActorForwardVector`) (* (`self.distance`) 100)))))
          (bind (_direction _newtrack_2) (`Timeline|Timeline`)
            (:`Update`
              (`self.K2_SetActorLocation` (`KismetMathLibrary.VLerp` (`self.K2_GetActorLocation`) _output_get_3 _newtrack_2)))))))))

(fn `UserConstructionScript`)